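; SpawnerController_BP is a controller that keeps a monster in the level by running the Spanwer_BT behavior tree.
; It runs the tree shortly after BeginPlay, then a looping timer checks every second whether any Monster_BP actor exists.
; When none is found, it pauses the timer, waits a random two to three-plus minutes, reruns the tree and resumes checking.
; RequestLocationAndRotation and RequestVariable only return default values.
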(event Custom|SpawnNewMonster
  (bind _returnvalue (Actor|GetActorOfClass "/Game/MyBlueprints/AI/Monster_BP.Monster_BP_C"))
  (if (not (Utilities|IsValid _returnvalue))
    (Utilities|Time|PauseTimerbyHandle (Variables|Default|GetIsDeadTimer))
    (Utilities|FlowControl|Delay (Math|Random|RandomFloatinRange 1.2e+02 2e+02))
    (AI|RunBehaviorTree "/Game/MyBlueprints/Objects/Spanwer_BT.Spanwer_BT")
    (Utilities|FlowControl|Delay 5.0)
    (Utilities|Time|UnpauseTimerbyHandle (Variables|Default|GetIsDeadTimer))))

(event EventBeginPlay
  (Utilities|FlowControl|Delay 3.5)
  (AI|RunBehaviorTree "/Game/MyBlueprints/Objects/Spanwer_BT.Spanwer_BT")
  (bind _returnvalue (Utilities|Time|SetTimerbyEvent (delegate Custom|SpawnNewMonster) 1.0 true))
  (Variables|Default|SetIsDeadTimer _returnvalue))

(fn ConstructionScript)

(fn RequestLocationandRotation
  (return "0, 0, 0" "0, 0, 0"))

(fn RequestVariable
  (return false))