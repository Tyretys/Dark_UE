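; AI monster character that takes damage, heals and dies through a DamageSystemComponent, which its health and damage functions forward to.
; Tick triggers a delayed small heal while health is low and writes the result back to Health.
; On death it stops AI logic, plays a stagger montage, then restarts logic and sets a blackboard force-despawn flag.
; It also sets walk speed on request and accumulates hit counts in the blackboard.
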(event Custom|OnDeath
  (bind _selfaicontroller (Variables|Default|GetSelfAIController))
  (AI|ClearFocus _selfaicontroller)
  (AI|Logic|StopLogic (Variables|/Script/AIModule.AIController|GetBrainComponent _selfaicontroller) "")
  (Animation|Montage|PlayMontage (Variables|Character|GetMesh) "/Game/MyBlueprints/AI/Animations/Montages/Stagger_Big.Stagger_Big"
    (:OnCompleted
      (AI|Logic|StartLogic (Variables|/Script/AIModule.AIController|GetBrainComponent (Variables|Default|GetSelfAIController)))
      (AI|Components|Blackboard|SetValueasBool (AI|GetBlackboard 0) (Utilities|Name|MakeLiteralName "ForceDespawn?") true))))

(event EventRequestGroundSpeed
  (params (NewGroundSpeed :type Float%20%28double-precision%29))
  (Variables|/Script/Engine.CharacterMovementComponent|SetMaxWalkSpeed (Variables|Character|GetCharacterMovement) NewGroundSpeed))

(event EventBeginPlay
  (bind _asmonster_controller (Utilities|Casting|CastToMonsterController (Pawn|GetController)))
  (Utilities|IsValid _asmonster_controller
    (:Is%20Valid
      (Variables|Default|SetSelfAIController _asmonster_controller))))

(event EventTick
  (params (DeltaSeconds :type Float%20%28single-precision%29))
  (if (<= (Variables|/Game/MyBlueprints/AI/DamageSystem_Component.DamageSystem_Component_C|GetHealth (Variables|Default|GetDamageSystem_Component)) 35.0)
    (Utilities|FlowControl|Delay 1.0)
    (bind _newhealth (Class|DamageInterface|Heal(Message) self 2.0))
    (Variables|/Game/MyBlueprints/AI/DamageSystem_Component.DamageSystem_Component_C|SetHealth (Variables|Default|GetDamageSystem_Component) _newhealth)))

(fn ConstructionScript
  (EventDispatchers|BindEventtoOnDeath (Variables|Default|GetDamageSystem_Component) (EventDispatchers|CreateEvent :!event Custom|OnDeath)))

(fn CountHits
  (params (HitNumber :type Byte :default 0))
  (bind _selfaicontroller (Variables|Default|GetSelfAIController))
  (bind _returnvalue (AI|GetBlackboard _selfaicontroller))
  (Class|BlackboardComponent|SetValueasInt _returnvalue (Utilities|Name|MakeLiteralName "HitNumber") (+ (Class|BlackboardComponent|GetValueasInt _returnvalue (Utilities|Name|MakeLiteralName "HitNumber")) (Math|Conversions|ToInteger(Byte) HitNumber)))
  (return))

(fn GetCurrentHealth
  (return (Variables|/Game/MyBlueprints/AI/DamageSystem_Component.DamageSystem_Component_C|GetHealth (Variables|Default|GetDamageSystem_Component))))

(fn GetMaxHealth
  (return (Variables|/Game/MyBlueprints/AI/DamageSystem_Component.DamageSystem_Component_C|GetMaxHealth (Variables|Default|GetDamageSystem_Component))))

(fn Heal
  (params (AmountHealed :type Float%20%28double-precision%29))
  (bind _newhealth (Default|Heal (Variables|Default|GetDamageSystem_Component) AmountHealed))
  (return _newhealth))

(fn RequestLocationandRotation
  (return "0, 0, 0" "0, 0, 0"))

(fn RequestVariable
  (return false))

(fn TakeDamage
  (params (DamageInfo :type S%20Damage%20Info%20Structure))
  (bind _wasdamaged_ (Default|TakeDamage (Variables|Default|GetDamageSystem_Component) DamageInfo))
  (return _wasdamaged_))